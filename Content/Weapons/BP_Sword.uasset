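; BP_Sword is a melee weapon actor that swings and deals flat damage to actors its hitbox touches, ignoring its owner.
; Swing, gated by an IsSwinging flag, enables the hitbox and plays a timeline that rotates the mesh, then disables the hitbox and resets the rotation.
; The hitbox stays collision-free outside swings, so overlaps only cause damage mid-swing.
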(event OnComponentBeginOverlap(Hitbox)
  (params (OverlappedComponent :type Primitive%20Component%20Object%20Reference) (OtherActor :type Actor%20Object%20Reference) (OtherComp :type Primitive%20Component%20Object%20Reference) (OtherBodyIndex :type Integer) (bFromSweep :type Boolean) (SweepResult :type Hit%20Result%20Structure%20%28by%20ref%29))
  (if (!= OtherActor (Components|GetOwner))
    (Game|Damage|ApplyDamage OtherActor 25.0 0 self)))

(event Custom|Swing
  (if (not (Variables|Default|GetbIsSwinging))
    (Variables|Default|SetbIsSwinging true)
    (Collision|SetCollisionEnabled (Variables|Default|GetHitbox) "QueryOnly")
    (bind _newtrack_0 (Timeline|SwingTL PlayFromStart)
      (:Update
        (Transformation|SetRelativeRotation (Variables|Default|GetMesh) (Math|Rotator|Lerp(Rotator) "0, 0, 0" "-90.000000,0.000000,0.000000" _newtrack_0) false false))
      (:Finished
        (Collision|SetCollisionEnabled (Variables|Default|GetHitbox) "NoCollision")
        (Variables|Default|SetbIsSwinging false)
        (Transformation|SetRelativeRotation (Variables|Default|GetMesh) "0, 0, 0" false false)))))

(event EventBeginPlay
  (Collision|SetCollisionEnabled (Variables|Default|GetHitbox) "NoCollision"))

(event Collision|EventActorBeginOverlap
  (params (OtherActor :type Actor%20Object%20Reference)))

(event EventTick
  (params (DeltaSeconds :type Float%20%28single-precision%29)))

(fn ConstructionScript)