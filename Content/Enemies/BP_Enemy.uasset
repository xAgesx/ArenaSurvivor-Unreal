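; BP_Enemy is an enemy actor with health that destroys itself when killed.
; Any damage reduces Health, and at zero or below it sets IsDead, which blocks further damage handling, then destroys the actor.
; BeginPlay starts a looping timer that fires the Chase event twice a second, but Chase is empty, so no movement logic exists here.
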(event Custom|Chase
  ;[0.15 0.15 0.15 0.5] Chase
)

(event EventBeginPlay
  ;[0.15 0.15 0.15 0.5] Chase
  (Utilities|Time|SetTimerbyEvent (delegate Custom|Chase) 0.5 true))

(event Collision|EventActorBeginOverlap
  (params (OtherActor :type Actor%20Object%20Reference)))

(event EventTick
  (params (DeltaSeconds :type Float%20%28single-precision%29)))

(event Game|Damage|EventAnyDamage
  (params (Damage :type Float%20%28single-precision%29) (DamageType :type Damage%20Type%20Object%20Reference) (InstigatedBy :type Controller%20Object%20Reference) (DamageCauser :type Actor%20Object%20Reference))
  ;[0.15 0.15 0.15 0.5] Take Damage
  (if (not (Variables|Default|GetbIsDead))
    (bind _output_get (Variables|Default|SetHealth (- (Variables|Default|GetHealth) Damage)))
    (if (<= _output_get 0.0)
      (Variables|Default|SetbIsDead true)
      (Actor|DestroyActor))))

(fn ConstructionScript)